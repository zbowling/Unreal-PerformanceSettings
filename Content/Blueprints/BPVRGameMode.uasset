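; VR game mode that prepares the player for head-mounted display play at startup.
; When an HMD is enabled, it sets a local-floor tracking origin and adds the XR input mapping context to the first player's Enhanced Input subsystem; otherwise it prints a warning.
; On EndPlay it sets CPU stress test workers to zero, since they would otherwise keep running in PIE.
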(event EventBeginPlay
  (if (Class|HeadMountedDisplayFunctionLibrary|IsHeadMountedDisplayEnabled)
    (Class|HeadMountedDisplayFunctionLibrary|SetTrackingOrigin "LocalFloor")
    (Input|AddMappingContext (PlayerController|LocalPlayerSubsystems|GetEnhancedInputLocalPlayerSubsystem (Game|GetPlayerController 0)) "/Game/Inputs/XR_InputMappingContext.XR_InputMappingContext" 0 "(bIgnoreAllPressedKeysUntilRelease=True,bForceImmediately=False,bNotifyUserSettings=False)")
    (Development|PrintString "Added Mapping Context")
    (else
      (Development|PrintString "Warning:Head mounted Display not enabled" true true "(R=0.000000,G=0.660000,B=1.000000,A=1.000000)" 1e+01))))

(event EventEndPlay
  (params (EndPlayReason :type EEndPlayReason%20Enum :default "Destroyed"))
  ;[0.15 0.15 0.15 0.5] in PIE these will keep running without this
  (Class|OUIBlueprintFunctionLibrary|SetNumCPUStressTestWorkers)
  (Development|PrintString "stopped all stress testers"))

(fn ConstructionScript)