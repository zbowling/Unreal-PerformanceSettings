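; A Blueprint function library of performance utilities that reads and adjusts XR rendering settings through console variables.
; Getters report anti-aliasing method (mapped to a name and validity flag), mobile forward shading and MSAA count.
; Render scale get and set switch between the HMD secondary screen percentage on UE 5.5 or later and pixel density on older engines.
; It also exposes lookup tables converting processor performance levels to and from strings.
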(fn GetAntiAliasingMethod
  (bind _returnvalue (Development|GetConsoleVariableIntValue "r.AntiAliasingMethod"))
  (bind _value (CallFunction|FindAntiAliasingMethodString _returnvalue))
  (bind _isvalid (CallFunction|IsAntiAliasingMethodValid _returnvalue))
  (return _value _isvalid))

(fn FindAntiAliasingMethodString
  (params (key :type Integer))
  (return (.Value (Utilities|Map|Find (LocalVariables|GetAntiAliasingMethodToString_0) key))))

(fn IsAntiAliasingMethodValid
  (params (Key :type Integer))
  (return (Utilities|Set|Contains (LocalVariables|GetValidAntiAliasingMethods_0) Key)))

(fn IsForwardShading
  (bind _returnvalue (Development|GetConsoleVariableIntValue "r.Mobile.ShadingPath"))
  (return (== _returnvalue 0)))

(fn GetMSAALevel
  (bind _returnvalue (Development|GetConsoleVariableIntValue "r.MSAACount"))
  (return _returnvalue))

(fn SetRenderScaleLevel
  (params (level :type Float%20%28double-precision%29))
  (if (Class|OUIBlueprintFunctionLibrary|IsUE55orLater)
    (Development|ExecuteConsoleCommand 0 (Utilities|String|ToString(Text) (Utilities|Text|FormatText "xr.SecondaryScreenPercentage.HMDRenderTarget {level}" (Class|KismetMathLibrary|ToInt64(Float) (* level 1e+02)))) 0)
    (else
      (Development|ExecuteConsoleCommand 0 (Utilities|String|ToString(Text) (Utilities|Text|FormatText "vr.PixelDensity {level}" level)) 0))))

(fn GetRenderScaleLevel
  (if (Class|OUIBlueprintFunctionLibrary|IsUE55orLater)
    (bind _returnvalue (Development|GetConsoleVariableIntValue "xr.SecondaryScreenPercentage.HMDRenderTarget"))
    (return (/ (Math|Conversions|ToFloat(Integer) _returnvalue) 1e+02))
    (else
      (bind _returnvalue_2 (Development|GetConsoleVariableFloatValue "vr.PixelDensity"))
      (return _returnvalue_2))))

(fn GetStringtoProcessorPerfLevels
  (return (LocalVariables|GetStringToCPULevel)))

(fn GetProcessorLevelstoString
  (return (LocalVariables|GetProcLevelsToString)))